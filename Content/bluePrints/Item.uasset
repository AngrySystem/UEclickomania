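; Clickable Item actor for a field-based game, shown as a sphere in one of three colors.
; On BeginPlay it applies a blue, green or red material to the sphere according to its Color value.
; A click passes the item to Field's OnitemClick, and the MoveTo event slides the sphere component to given relative coordinates over a short time.
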(event `self.ReceiveBeginPlay`
  (bind _sphere (`self.Sphere`))
  (switch `int` (`self.Color`)
    (:`0`
      (`PrimitiveComponent.SetMaterial` _sphere 0 "/Game/Materials/Blue.Blue"))
    (:`1`
      (`PrimitiveComponent.SetMaterial` _sphere 0 "/Game/Materials/green.green"))
    (:`2`
      (`PrimitiveComponent.SetMaterial` _sphere 0 "/Game/Materials/red.red"))))

(event `self.ReceiveActorOnClicked`
  (params (ButtonPressed :type "Key Structure"))
  (`/Game/bluePrints/field.OnitemClick` (`self.Field`) self))

(event `MoveTo`
  (params (cords :type "Vector Structure"))
  (`KismetSystemLibrary.MoveComponentTo` (`self.Sphere`) cords (struct) false false 0.5))

(fn `UserConstructionScript`)